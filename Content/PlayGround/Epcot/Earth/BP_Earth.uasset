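; Interactive Epcot Earth globe that spins on its own and can be turned by one touching VR hand at a time, synced across multiplayer.
; Touch attaches the sphere to a pivot following the hand, optionally carrying the sun; release eases the measured speed back to idle spin.
; The server relays rotation and controlling player, and halts idle spin when hands come close.
; An opacity timeline fades the globe and toggles the EarthCity UI system.
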(event Custom|SetSelfRotateEnable
  (params (bEnabled :type Boolean))
  (if (and (not (Networking|IsServer)) (not (Utilities|IsValid (Variables|Default|GetcurTouchingHand))))
    (Actor|Tick|SetActorTickEnabled bEnabled)
    (Development|PrintString (Utilities|String|Append "Self rotate enable (tick enable): " (Utilities|String|ToString(Boolean) bEnabled)))))

(event Custom|FadeInOut
  (params (IsIn :type Boolean) (Rate :type Float%20%28double-precision%29))
  (Components|Timeline|SetPlayRate (Variables|Default|GetTimeline_Opacity) Rate)
  (if IsIn
    (Class|CommonFunctionLibrary|SetActiveAdvanced self true false true)
    (bind _opacity (Timeline|Timeline_Opacity Play)
      (:Update
        (Rendering|Material|SetScalarParameterValue (Variables|Default|GetDynMatInst) "Opacity Mask" _opacity :!class /Script/Engine.MaterialInstanceDynamic))
      (:Finished
        (Class|CommonFunctionLibrary|SetActiveAdvanced self IsIn IsIn IsIn)
        (Utilities|FlowControl|Sequence
          (:then_0
            (bind _gamesystem (CallFunction|GetGameSystem "Epcot" "EarthCityUISystem"))
            (Utilities|IsValid _gamesystem
              (:Is%20Valid
                (Actor|Tick|SetActorTickEnabled _gamesystem IsIn)
                (Class|ELSystemBase|SetEnable _gamesystem IsIn))))
          (:then_1
            (if IsIn
              (bind _outactors (Actor|GetAllActorsOfClass "/ELGameFramework/Hand/ELHandBase.ELHandBase_C"))
              (Variables|Default|SetallHands _outactors)
              (else
                (Default|ResettoInitState (Actor|GetComponentsByClass "/Game/PlayGround/Epcot/Component/EarthCityComponent.EarthCityComponent_C"))))))))
    (else
      (Timeline|Timeline_Opacity Reverse))))

(event Custom|SyncRotateCenter
  (params (NewRotation :type Rotator))
  (Variables|Default|GetcurTouchingHand
    (:then)
    (:else
      (Transformation|SetWorldRotation (Variables|Default|GetRotateCenter) NewRotation false false)
      (Development|PrintString "Client sync rotation center."))))

(event Custom|UpdateRotationByTouchingHand
  (params (deltaSec :type Float%20%28double-precision%29))
  (bind _curtouchinghand (Variables|Default|GetcurTouchingHand)
    (:then
      (Variables|Default|SetRotateSpeed_Touching (/ (.yaw (Math|Rotator|Delta(Rotator) (Math|Rotator|MakeRotfromZX (Math|Vector|MakeVector 0.0 0.0 1.0) (- (Transformation|GetWorldLocation (Variables|/ELGameFramework/Hand/ELHandBase.ELHandBase_C|GetHandCenter _curtouchinghand)) (Transformation|GetWorldLocation (Variables|Default|GetSphere_Earth)))) (Variables|Default|GetCurRot_Touch))) deltaSec))
      (bind _output_get (Variables|Default|SetCurRot_Touch (Math|Rotator|MakeRotfromZX (Math|Vector|MakeVector 0.0 0.0 1.0) (- (Transformation|GetWorldLocation (Variables|/ELGameFramework/Hand/ELHandBase.ELHandBase_C|GetHandCenter _curtouchinghand)) (Transformation|GetWorldLocation (Variables|Default|GetSphere_Earth))))))
      (Transformation|SetWorldRotation (Variables|Default|GetRotateCenter) _output_get false false)
      (Utilities|FlowControl|Sequence
        (:then_0
          (if (Utilities|IsLeftHandtoRotateSun)
            (bind _sunactor (Variables|Default|GetSunActor)
              (:then
                (Default|SetupSunDirectiontoMaterialCollection _sunactor))
              (:else))))
        (:then_1
          (if (Networking|IsServer)
            (CallFunction|UpdateRotationtoClient (Variables|Default|GetCurRot_Touch))))))
    (:else)))

(event Custom|UpdateRotationToClient
  (params (New%20Rotation :type Rotator))
  (Variables|Default|GetcurTouchingHand
    (:then)
    (:else
      (Transformation|SetWorldRotation (Variables|Default|GetRotateCenter) New%20Rotation false false))))

(event Custom|AttachEarthToRotateCenter
  (params (AttachToRotateCenter :type Boolean) (RotateSun :type Boolean))
  (Transformation|AttachComponentToComponent (Variables|Default|GetSphere_Earth) (select AttachToRotateCenter (Variables|Default|GetRotateCenter) (Variables|Default|GetDefaultSceneRoot)) "None" "SnapToTarget" "KeepWorld" "KeepWorld" true)
  (Development|PrintString (Utilities|String|Append "Attach to rotate center: " (Utilities|String|ToString(Boolean) AttachToRotateCenter)))
  (if RotateSun
    (bind _sunactor (Variables|Default|GetSunActor)
      (:then
        (Transformation|AttachComponentToComponent _sunactor (select AttachToRotateCenter (Variables|Default|GetRotateCenter) (Variables|Default|GetDefaultSceneRoot)) "None" "KeepWorld" "KeepWorld" "KeepWorld" true))
      (:else))))

(event Custom|AttachEarthToRotateCenter_Multicast
  (params (AttachToRotateCenter :type Boolean) (RotateSun :type Boolean))
  (CallFunction|AttachEarthtoRotateCenter AttachToRotateCenter RotateSun))

(event Custom|SetupControllingPlayerToClient
  (params (controllingPlayer :type Pawn%20Object%20Reference))
  (bind _output_get (Variables|Default|SetcontrollingPlayer controllingPlayer))
  (Utilities|IsValid _output_get
    (:Is%20Valid
      (if (not (Networking|IsServer))
        (if (not (== (Variables|Default|GetcontrollingPlayer) (Game|Player|GetPlayerPawn 0)))
          (Variables|Default|SetcurTouchingHand 0)
          (CallFunction|SetSelfRotateEnable false))))))

(event Custom|UpdateRotateSpeed
  (params (RotateSpeed :type Float%20%28double-precision%29))
  (bind _output_get (Variables|Default|SetRotateSpeed RotateSpeed)))

(event Custom|UpdateRotateSpeedTouchingToClient
  (params (NewRotateSpeed_Touching :type Float%20%28double-precision%29))
  (bind _output_get (Variables|Default|SetRotateSpeed_Touching NewRotateSpeed_Touching))
  (Development|PrintString (Utilities|String|Append "Client update rotate speed touching" (Utilities|String|ToString(Float) _output_get))))

(event EventBeginPlay
  (Variables|Default|SetRotate%20Speed_Init (Variables|Default|GetRotateSpeed))
  (bind _returnvalue (Rendering|Material|CreateDynamicMaterialInstance (Variables|Default|GetSphere_Earth) 0 "/Game/PlayGround/Epcot/Earth/Material/Earth_M_Inst.Earth_M_Inst" "None" :!class /Script/Engine.PrimitiveComponent))
  (Variables|Default|SetDynMatInst _returnvalue)
  (Class|CommonFunctionLibrary|SetActiveAdvanced self false false false))

(event EventOnBeginTouched
  (params (Hand :type EL%20Hand%20Base%20Object%20Reference))
  (Variables|Default|GetcurTouchingHand
    (:then)
    (:else
      (Variables|Default|SetcurTouchingHand Hand)
      (Variables|Default|SetCurRot_Touch (Transformation|GetWorldRotation (Variables|Default|GetRotateCenter)))
      (Utilities|FlowControl|Sequence
        (:then_0
          (CallFunction|UpdateRotationbyTouchingHand 1e-05)
          (if (Networking|IsServer)
            (CallFunction|SyncRotateCenter (Transformation|GetWorldRotation (Variables|Default|GetRotateCenter)))))
        (:then_1
          (if (Networking|IsServer)
            (bind _aspawn (Utilities|Casting|CastToPawn (Actor|GetAttachParentActor (Variables|Default|GetcurTouchingHand))))
            (bind _output_get (Variables|Default|SetcontrollingPlayer _aspawn))
            (CallFunction|SetupControllingPlayertoClient _output_get)
            (CallFunction|SetSelfRotateEnable false)
            (CallFunction|AttachEarthtoRotateCenterMulticast true (Utilities|IsLeftHandtoRotateSun))
            (else
              (CallFunction|AttachEarthtoRotateCenter true (Utilities|IsLeftHandtoRotateSun)))))))))

(event EventTick
  (params (DeltaSeconds :type Float%20%28single-precision%29))
  (Utilities|FlowControl|Sequence
    (:then_0
      (Variables|Default|GetcurTouchingHand
        (:then
          (CallFunction|UpdateRotationbyTouchingHand DeltaSeconds))
        (:else
          (bind _output_get (Variables|Default|SetRotateSpeed_Touching (Math|Interpolation|FInterpTo (Variables|Default|GetRotateSpeed_Touching) (Variables|Default|GetRotateSpeed) DeltaSeconds 1.0)))
          (Transformation|AddLocalRotation (Variables|Default|GetSphere_Earth) (Math|Rotator|MakeRotator 0.0 0.0 (* _output_get DeltaSeconds)) false false))))
    (:then_1
      (if (Networking|IsServer)
        (bind _returnvalue (CallFunction|CheckAnyHandClosed))
        (if (!= _returnvalue (Variables|Default|GethandIsClosed))
          (bind _output_get_2 (Variables|Default|SethandIsClosed _returnvalue))
          (CallFunction|UpdateRotateSpeed (Math|Float|SelectFloat 0.0 (Variables|Default|GetRotate%20Speed_Init) _output_get_2)))))))

(event EventOnEndTouched
  (params (Hand :type EL%20Hand%20Base%20Object%20Reference))
  (if (== Hand (Variables|Default|GetcurTouchingHand))
    (if (Networking|IsServer)
      (CallFunction|AttachEarthtoRotateCenterMulticast false (Utilities|IsLeftHandtoRotateSun))
      (CallFunction|SyncRotateCenter (Transformation|GetWorldRotation (Variables|Default|GetRotateCenter)))
      (CallFunction|UpdateRotateSpeedTouchingtoClient (Variables|Default|GetRotateSpeed_Touching))
      (CallFunction|SetSelfRotateEnable true)
      (Variables|Default|SetcontrollingPlayer 0)
      (CallFunction|SetupControllingPlayertoClient)
      (Variables|Default|SetcurTouchingHand 0)
      (else
        (Variables|Default|SetcurTouchingHand 0)))))

(fn ConstructionScript)

(fn CheckAnyHandClosed
  (for _array_element (Variables|Default|GetallHands)
    (if (<= (- (Math|Vector|VectorLength (- (Transformation|GetWorldLocation (Variables|/ELGameFramework/Hand/ELHandBase.ELHandBase_C|GetHandCenter _array_element)) (Transformation|GetActorLocation))) (.SphereRadius (Collision|GetComponentBounds (Variables|Default|GetSphere_Earth)))) (Variables|Default|GetclosedDistance))
      (return true)))
  (return false))

(fn CanInteract
  (params (InteractWithActor :type Actor%20Object%20Reference))
  (return (not (Utilities|IsValid (Variables|Default|GetcurTouchingHand)))))

(fn ScaleColliderwhenOverlapped
  (return false))