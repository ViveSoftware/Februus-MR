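; Helper actor that supplies the sun direction for the Earth materials in the Epcot playground.
; It writes its own world location, unnormalized, as the SunDirection vector in EarthMaterialCollection, so the actor's position relative to the world origin defines the direction.
; The construction script pushes the value, and BeginPlay can push it again when SetupSunDirectionOnBeginPlay is enabled.
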(event Custom|SetupSunDirectionToMaterialCollection
  (Rendering|Material|SetVectorParameterValue "/Game/PlayGround/Epcot/Earth/Material/EarthMaterialCollection.EarthMaterialCollection" "SunDirection" (Math|Conversions|ToLinearColor(Vector) (Transformation|GetActorLocation)) :!class /Script/Engine.KismetMaterialLibrary))

(event EventBeginPlay
  (if (Variables|Default|GetSetupSunDirectionOnBeginPlay)
    (CallFunction|SetupSunDirectiontoMaterialCollection)))

(fn ConstructionScript
  (Rendering|Material|SetVectorParameterValue "/Game/PlayGround/Epcot/Earth/Material/EarthMaterialCollection.EarthMaterialCollection" "SunDirection" (Math|Conversions|ToLinearColor(Vector) (Transformation|GetActorLocation)) :!class /Script/Engine.KismetMaterialLibrary))