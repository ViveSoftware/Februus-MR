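; BP_ScalablePointLight is a point light actor whose brightness and reach follow the actor's X scale.
; After a configurable delay on BeginPlay, it multiplies the light's intensity and attenuation radius by that scale.
; StartPointLightCurve resets the timer and enables Tick, which sets intensity from IntensityCurve over elapsed time, multiplied by the X scale.
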(event Custom|StartPointLightCurve
  (Variables|Default|SetcurTime 0.0)
  (Actor|Tick|SetActorTickEnabled true))

(event EventTick
  (params (DeltaSeconds :type Float%20%28single-precision%29))
  (bind _output_get (Variables|Default|SetcurTime (+ (Variables|Default|GetcurTime) DeltaSeconds)))
  (Rendering|Components|Light|SetIntensity (Variables|Default|GetPointLight) (* (Math|Curves|GetFloatValue (Variables|Default|GetIntensityCurve) _output_get) (.x (Transformation|GetActorScale3D)))))

(event EventBeginPlay
  (bind _returnvalue (Transformation|GetActorScale3D))
  (bind _pointlight (Variables|Default|GetPointLight))
  (Utilities|FlowControl|Delay (Variables|Default|GetBeginPlayDelayDuration))
  (Rendering|Components|Light|SetIntensity _pointlight (* (.x _returnvalue) (Variables|/Script/Engine.LightComponentBase|GetIntensity _pointlight)))
  (Rendering|Lighting|SetAttenuationRadius _pointlight (* (.x _returnvalue) (Variables|/Script/Engine.LocalLightComponent|GetAttenuationRadius _pointlight))))

(fn ConstructionScript)