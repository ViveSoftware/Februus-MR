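; BP_EarthButton is an interactive pin button on the Epcot Earth, tied to a city component.
; Its construction script wires the button and hover spheres, circular gauge and pin root into EarthCityComp, which receives them as its collider and UI references.
; The pin root is also the target of a SinFloatingComponent, whose tick is enabled at BeginPlay to float the pin.
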(event EventBeginPlay
  (Components|Tick|SetComponentTickEnabled (Variables|Default|GetSinFloatingComponent) true))

(fn ConstructionScript
  (Utilities|FlowControl|Sequence
    (:then_0
      (bind _earthcitycomp (Variables|Default|GetEarthCityComp)
        (:then
          (Variables|/Game/PlayGround/Epcot/Component/EarthCityComponent.EarthCityComponent_C|SetCollider _earthcitycomp (Variables|Default|GetSphereButton))
          (Variables|/Game/PlayGround/Epcot/Component/EarthCityComponent.EarthCityComponent_C|SetUI_CircularGauge _earthcitycomp (Variables|Default|GetCircularGauge))
          (Variables|/Game/PlayGround/Epcot/Component/EarthCityComponent.EarthCityComponent_C|SetCollider_Hover _earthcitycomp (Variables|Default|GetSphereButton_Hover))
          (Variables|/Game/PlayGround/Epcot/Component/EarthCityComponent.EarthCityComponent_C|SetUI_Pin _earthcitycomp (Variables|Default|Getpin_root)))
        (:else)))
    (:then_1
      (Variables|/ELGameFramework/Components/SinFloatingComponent.SinFloatingComponent_C|Setcomponent (Variables|Default|GetSinFloatingComponent) (Variables|Default|Getpin_root)))))