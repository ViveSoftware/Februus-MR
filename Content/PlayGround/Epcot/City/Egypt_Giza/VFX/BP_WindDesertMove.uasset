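; Desert wind VFX actor for the Giza city that sweeps a particle emitter along a straight path when StartMoving runs.
; TargetActor's bounds set path length and width.
; Tick advances a center point at constant speed, teleporting the emitter to random offsets around it to cover a moving band, then deactivates at the end.
; The attach parent's EarthCitySizeControlComponent broadcasts scale changes that rescale path, band, speed and particle parameters.
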(event Custom|StartMoving
  (bind _movedirection (Variables|Default|GetMoveDirection))
  (Utilities|FlowControl|Sequence
    (:then_0
      (Variables|Default|SetSpawnWidthVector (Math|Vector|GetRightVector _movedirection))
      (bind _output_get (Variables|Default|SetEndLocation (+ (Transformation|GetActorLocation) (* (Math|Vector|GetForwardVector _movedirection) (Variables|Default|GetMovePathLength))))))
    (:then_1
      (bind _output_get_2 (Variables|Default|SetCurCenter (Transformation|GetActorLocation)))
      (Transformation|SetWorldLocation (Variables|Default|GetWindDesert_Point) _output_get_2 false true)
      (Actor|Tick|SetActorTickEnabled true)
      (Components|Activation|SetActive (Variables|Default|GetWindDesert_Point) true true))))

(event Custom|OnEarthCitySizeChanged_Event
  (params (New%20location :type Vector) (New%20rotation :type Rotator) (New%20scale :type Vector))
  (bind _x (Class|KismetMathLibrary|BreakVector3f New%20scale))
  (bind _winddesert_point (Variables|Default|GetWindDesert_Point))
  (Utilities|FlowControl|Sequence
    (:then_0
      (Effects|Components|ParticleSystem|SetFloatParameter _winddesert_point "ScaleSpriteCurve" (* _x (Variables|Default|GetParticleScaleSpriteCurve)))
      (Effects|Components|ParticleSystem|SetFloatParameter _winddesert_point "CurlNoiseForceStrength" (* _x (Variables|Default|GetParticleCurlNoiseForceStrength)))
      (Effects|Components|ParticleSystem|SetFloatParameter _winddesert_point "ScaleVelocity" _x))
    (:then_1
      (Variables|Default|SetSpawnHalfWidth (* _x (Variables|Default|GetSpawnHalfWidth_Original)))
      (Variables|Default|SetSpawnHalfHeight (* _x (Variables|Default|GetSpawnHalfHeight_Original)))
      (Variables|Default|SetMovePathLength (* _x (Variables|Default|GetMovePathLength_Original)))
      (Variables|Default|SetMoveSpeed (* _x (Variables|Default|GetMoveSpeed_Original))))))

(event EventBeginPlay
  (bind _targetactor (Variables|Default|GetTargetActor))
  (bind _winddesert_point (Variables|Default|GetWindDesert_Point))
  (bind _defaultsceneroot (Variables|Default|GetDefaultSceneRoot))
  (bind _returnvalue (Transformation|GetAttachParent _defaultsceneroot))
  (bind _boxextent (Collision|GetActorBounds _targetactor false false))
  (bind _returnvalue_2 (Components|GetOwner _returnvalue))
  (bind _returnvalue_3 (Actor|GetComponentbyClass _returnvalue_2 "/Game/PlayGround/Epcot/Component/EarthCitySizeControlComponent.EarthCitySizeControlComponent_C"))
  (Utilities|FlowControl|Sequence
    (:then_0
      (bind _output_get (Variables|Default|SetMovePathLength (* (.y _boxextent) 2.0)))
      (Variables|Default|SetMovePathLength_Original _output_get)
      (bind _output_get_2 (Variables|Default|SetSpawnHalfWidth (.x _boxextent)))
      (Variables|Default|SetSpawnHalfWidth_Original _output_get_2)
      (Variables|Default|SetMoveSpeed_Original (Variables|Default|GetMoveSpeed))
      (Effects|Components|ParticleSystem|SetFloatParameter _winddesert_point "ScaleSpriteCurve" (Variables|Default|GetParticleScaleSpriteCurve))
      (Effects|Components|ParticleSystem|SetFloatParameter _winddesert_point "CurlNoiseForceStrength" (Variables|Default|GetParticleCurlNoiseForceStrength)))
    (:then_1
      (Utilities|IsValid _returnvalue_2
        (:Is%20Valid
          (Utilities|IsValid _returnvalue_3
            (:Is%20Valid
              (EventDispatchers|AssignOnEarthCitySizeChanged _returnvalue_3 (delegate Custom|OnEarthCitySizeChanged_Event)))
            (:Is%20Not%20Valid
              (Development|PrintString "No earth city size control component."))))))))

(event EventTick
  (params (DeltaSeconds :type Float%20%28single-precision%29))
  (bind _returnvalue (Math|Random|RandomFloatinRange -1.0 1.0))
  (bind _spawnwidthvector (Variables|Default|GetSpawnWidthVector))
  (bind _spawnhalfwidth (Variables|Default|GetSpawnHalfWidth))
  (bind _returnvalue_2 (* _spawnhalfwidth _returnvalue))
  (bind _returnvalue_3 (* _spawnwidthvector _returnvalue_2))
  (Variables|Default|SetCurCenter (Math|Interpolation|VInterptoConstant (Variables|Default|GetCurCenter) (Variables|Default|GetEndLocation) DeltaSeconds (Variables|Default|GetMoveSpeed)))
  (Transformation|SetWorldLocation (Variables|Default|GetWindDesert_Point) (+ (Variables|Default|GetCurCenter) (Math|Vector|MakeVector (.x _returnvalue_3) (.y _returnvalue_3) (* (Variables|Default|GetSpawnHalfHeight) _returnvalue))) false true)
  (if (Utilities|Operators|EqualEqual (Variables|Default|GetCurCenter) (Variables|Default|GetEndLocation) 0.1)
    (Actor|Tick|SetActorTickEnabled false)
    (Components|Activation|SetActive (Variables|Default|GetWindDesert_Point) false false)))

(fn ConstructionScript)