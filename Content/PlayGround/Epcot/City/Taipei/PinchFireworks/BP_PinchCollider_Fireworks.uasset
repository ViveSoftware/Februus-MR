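; Timed pinch target for the fireworks interaction, showing billboarded circular gauges and reporting whether the hand pinch succeeded.
; PrepareCountDown plays a delayed, gate-cancelable intro ring animation, while StartCountDown runs a timeline that fills the gauge.
; A timeline event opens the pinch gate, so only a pinch inside that window spawns the burst and marks success.
; Countdown end, or Reset while in use, reports the result through CallPinchFinshed.
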(event Custom|CloseCheckIsPinchGate
  (Utilities|FlowControl|Gate true) ; enters at Close
)

(event Custom|OpenCheckIsPinchGate
  (Utilities|FlowControl|Gate true) ; enters at Open
)

(event Custom|StartCountDown
  (bind _circulargaugedynmatinst (Variables|Default|GetCircularGaugeDynMatInst))
  (Rendering|SetActorHiddenInGame false)
  (Collision|SetActorEnableCollision true)
  (bind _circulargauge (Timeline|CountDownPinch PlayFromStart)
    (:Update
      (Rendering|Material|SetScalarParameterValue _circulargaugedynmatinst "Decimal" _circulargauge :!class /Script/Engine.MaterialInstanceDynamic)
      (Rendering|Material|SetScalarParameterValue _circulargaugedynmatinst "EmissiveScale" (* _circulargauge 1e+01) :!class /Script/Engine.MaterialInstanceDynamic))
    (:Finished
      (Utilities|FlowControl|RetriggerableDelay 0.5)
      (CallFunction|CloseCheckIsPinchGate)
      (Development|PrintString (Utilities|String|Append (Utilities|GetDisplayName self) " pinch success: " (Utilities|String|ToString(Boolean) (Variables|Default|GetSuccess))))
      (Rendering|SetActorHiddenInGame true)
      (Collision|SetActorEnableCollision false)
      (Variables|Default|SetinUse false)
      (Utilities|FlowControl|Sequence
        (:then_0
          (if (Variables|Default|GetSuccess)
            _))
        (:then_1
          (Default|CallPinchFinshed self (Variables|Default|GetSuccess)))))
    (:OpenPinchGate
      (CallFunction|OpenCheckIsPinchGate))))

(event Custom|PrepareCountDown
  (params (DelayDuration :type Float%20%28double-precision%29))
  (Variables|Default|SetinUse true)
  (Variables|Default|SetSuccess false)
  (CallFunction|CloseCheckIsPinchGate)
  (Rendering|Material|SetScalarParameterValue (Variables|Default|GetCircularGaugeDynMatInst) "Decimal" 0.0 :!class /Script/Engine.MaterialInstanceDynamic)
  (Utilities|FlowControl|Sequence
    (:then_0
      (Utilities|FlowControl|Delay DelayDuration)
      (Utilities|FlowControl|Gate true :!label _label
        (:Exit
          (Rendering|SetActorHiddenInGame false)
          (Components|Timeline|SetPlayRate (Variables|Default|GetPrepareAnimation) 0.8)
          (bind (_direction _scale _thickness) (Timeline|PrepareAnimation PlayFromStart)
            (:Update
              (Transformation|SetRelativeScale3D (Variables|Default|GetPlane_CircularGauge_Prepare) (Math|Vector|MakeVector _scale _scale _scale))
              (Rendering|Material|SetScalarParameterValue (Variables|Default|GetCircularGaugeDynMatInst_Prepare) "Thickness" _thickness :!class /Script/Engine.MaterialInstanceDynamic))))))
    (:then_1
      (goto _label Open))))

(event Custom|Reset
  (Utilities|FlowControl|Sequence
    (:then_0
      (if (Variables|Default|GetinUse)
        (Default|CallPinchFinshed self (Variables|Default|GetSuccess))))
    (:then_1
      (CallFunction|StopAllTimeline)
      (Variables|Default|SetinUse false)
      (Variables|Default|SetSuccess false))))

(event Custom|StopAllTimeline
  (bind _circulargaugedynmatinst (Variables|Default|GetCircularGaugeDynMatInst))
  (Utilities|FlowControl|Sequence
    (:then_0
      (bind _circulargauge (Timeline|CountDownPinch Stop)
        (:Update
          (Rendering|Material|SetScalarParameterValue _circulargaugedynmatinst "Decimal" _circulargauge :!class /Script/Engine.MaterialInstanceDynamic)
          (Rendering|Material|SetScalarParameterValue _circulargaugedynmatinst "EmissiveScale" (* _circulargauge 1e+01) :!class /Script/Engine.MaterialInstanceDynamic))
        (:Finished
          (Utilities|FlowControl|RetriggerableDelay 0.5)
          (CallFunction|CloseCheckIsPinchGate)
          (Development|PrintString (Utilities|String|Append (Utilities|GetDisplayName self) " pinch success: " (Utilities|String|ToString(Boolean) (Variables|Default|GetSuccess))))
          (Rendering|SetActorHiddenInGame true)
          (Collision|SetActorEnableCollision false)
          (Variables|Default|SetinUse false)
          (Utilities|FlowControl|Sequence
            (:then_0
              (if (Variables|Default|GetSuccess)
                _))
            (:then_1
              (Default|CallPinchFinshed self (Variables|Default|GetSuccess)))))
        (:OpenPinchGate
          (CallFunction|OpenCheckIsPinchGate))))
    (:then_1
      (bind (_direction _scale _thickness) (Timeline|PrepareAnimation Stop)
        (:Update
          (Transformation|SetRelativeScale3D (Variables|Default|GetPlane_CircularGauge_Prepare) (Math|Vector|MakeVector _scale _scale _scale))
          (Rendering|Material|SetScalarParameterValue (Variables|Default|GetCircularGaugeDynMatInst_Prepare) "Thickness" _thickness :!class /Script/Engine.MaterialInstanceDynamic))))
    (:then_2
      (Utilities|FlowControl|Gate true) ; enters at Close
    )))

(event EventBeginPlay
  (|CallParentFunction)
  (bind _returnvalue (Rendering|Material|CreateDynamicMaterialInstance (Variables|Default|GetPlane_CircularGauge) 0 "/ELGameFramework/Materials/CircleGauge/CircleGaugeMat_Blue.CircleGaugeMat_Blue" "None" :!class /Script/Engine.PrimitiveComponent))
  (bind _output_get (Variables|Default|SetCircularGaugeDynMatInst _returnvalue))
  (Rendering|Material|SetScalarParameterValue _output_get "Thickness" 0.2 :!class /Script/Engine.MaterialInstanceDynamic)
  (Rendering|Material|SetScalarParameterValue _output_get "EmissiveScale" 2.0 :!class /Script/Engine.MaterialInstanceDynamic)
  (Rendering|Material|SetScalarParameterValue _output_get "Decimal" 0.0 :!class /Script/Engine.MaterialInstanceDynamic)
  (Rendering|SetActorHiddenInGame true)
  (bind _returnvalue_2 (Rendering|Material|CreateDynamicMaterialInstance (Variables|Default|GetPlane_CircularGauge_Prepare) 0 "/ELGameFramework/Materials/CircleGauge/CircleGaugeMat_White.CircleGaugeMat_White" "None" :!class /Script/Engine.PrimitiveComponent))
  (Variables|Default|SetCircularGaugeDynMatInst_Prepare _returnvalue_2))

(event EventCallonPinchCollider
  (params (Hand :type EControllerHand%20Enum :default "Left"))
  (Utilities|FlowControl|Gate true
    (:Exit
      (|CallParentFunction Hand)
      (Rendering|SetActorHiddenInGame true)
      (Effects|SpawnEmitteratLocation "/Game/PlayGround/Epcot/City/Taipei/VFX/PS_TS_Fireworks_Burst_Palm1.PS_TS_Fireworks_Burst_Palm1" (Transformation|GetActorLocation))
      (CallFunction|CloseCheckIsPinchGate)
      (Variables|Default|SetSuccess true))))

(fn ConstructionScript
  (|CallParentFunction)
  (Variables|/ELGameFramework/Components/BillboardComponent.BillboardComponent_C|SetBillboardsComponents (Variables|Default|GetBillboardComponent) (Utilities|Array|MakeArray (Variables|Default|GetCircularGaugeRoot))))