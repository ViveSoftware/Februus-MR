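; Locator actor for the Taipei pinch fireworks that positions pinch colliders in front of the player's camera, toward the Earth actor.
; On setup it moves and billboards itself, then assigns colliders to randomly shuffled free location slots.
; Each slot is released when its collider's pinch-finished event fires.
; A box counts overlapping fingertip colliders to toggle the playground selector's left-hand show-up binding off while fingers are inside.
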(event OnComponentBeginOverlap(Box)
  (params (OverlappedComponent :type Primitive%20Component%20Object%20Reference) (OtherActor :type Actor%20Object%20Reference) (OtherComp :type Primitive%20Component%20Object%20Reference) (OtherBodyIndex :type Integer) (bFromSweep :type Boolean) (SweepResult :type Hit%20Result%20Structure%20%28by%20ref%29))
  (Utilities|Casting|CastToELFingerTipCollider OtherActor)
  (Math|Integer|IncrementInt (Variables|Default|GetFingerOverlapNum)
    (:%20%20
      (Default|BindLeffHandShowUp (Variables|Default|GetBP_UI_PlaygeoundSelector) false))))

(event OnComponentEndOverlap(Box)
  (params (OverlappedComponent :type Primitive%20Component%20Object%20Reference) (OtherActor :type Actor%20Object%20Reference) (OtherComp :type Primitive%20Component%20Object%20Reference) (OtherBodyIndex :type Integer))
  (Utilities|Casting|CastToELFingerTipCollider OtherActor)
  (bind _result (Math|Integer|DecrementInt (Variables|Default|GetFingerOverlapNum))
    (:%20%20
      (if (== _result 0)
        (Default|BindLeffHandShowUp (Variables|Default|GetBP_UI_PlaygeoundSelector) true)))))

(event Custom|SetupPinchColliderLocation
  (params (pinchColliders :type Array%20of%20BP%20Pinch%20Collider%20Fireworks%20Object%20References))
  (bind _indexarr (Variables|Default|GetIndexArr))
  (bind _inusedarr (Variables|Default|GetInUsedArr))
  (Utilities|FlowControl|Sequence
    (:then_0
      (Variables|Default|SetPinchColliderAmount_Placed 0)
      (Variables|Default|SetPinchColliderAmount (Utilities|Array|Length pinchColliders))
      (bind _earthbp (Variables|Default|GetEarthBP)
        (:then
          (bind _camera (CallFunction|GetPawnCamera))
          (Transformation|SetActorLocation (+ (Transformation|GetWorldLocation _camera) (* (Math|Vector|Normalize (- (+ (Transformation|GetActorLocation _earthbp) "0, 0,-10.000000") (Transformation|GetWorldLocation _camera))) 55.0)) false true))
        (:else)))
    (:then_1
      (CallFunction|ActorBillboard self true false)
      (Utilities|Array|Shuffle _indexarr)
      (bind _array_element (Utilities|Array|ForEachLoopwithBreak _indexarr :!label _label)
        (:LoopBody
          (if (not (Utilities|Array|Get(acopy) _inusedarr _array_element))
            (Utilities|Array|SetArrayElem _inusedarr _array_element true)
            (Utilities|Map|Add (Variables|Default|GetPinchColliderToIndex) (Utilities|Array|Get(acopy) pinchColliders (Variables|Default|GetPinchColliderAmount_Placed)) _array_element)
            (Transformation|SetActorLocation (Utilities|Array|Get(acopy) pinchColliders (Variables|Default|GetPinchColliderAmount_Placed)) (Utilities|GetLoc _array_element) false true)
            (EventDispatchers|AssignPinchFinshed (Utilities|Array|Get(acopy) pinchColliders (Variables|Default|GetPinchColliderAmount_Placed)) (delegate Custom|PinchFinshed_Event))
            (bind _result (Math|Integer|IncrementInt (Variables|Default|GetPinchColliderAmount_Placed))
              (:%20%20
                (if (== _result (Variables|Default|GetPinchColliderAmount))
                  (goto _label Break))))))))))

(event Custom|PinchFinshed_Event
  (params (pinchCollider :type BP%20Pinch%20Collider%20Fireworks%20Object%20Reference) (Success :type Boolean))
  (EventDispatchers|UnbindEventfromPinchFinshed pinchCollider (delegate Custom|PinchFinshed_Event))
  (Utilities|Array|SetArrayElem (Variables|Default|GetInUsedArr) (.Value (Utilities|Map|Find (Variables|Default|GetPinchColliderToIndex) pinchCollider)) false))

(fn ConstructionScript)