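; Easter Island city actor that drives grass wind and cloud Niagara particles, responding to Earth city size changes.
; Size changes multiply the stored wind intensity by the new X scale, rescale the clouds, then activate them and start gusts after a delay.
; Each gust randomizes the MPC_GrassWind direction, sets cloud wind from actor orientation, and animates intensity by timeline before scheduling the next.
; EndPlay restores the original intensity and zeroes the wind vector.
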(event Custom|OnEarthCitySizeChanged_Event
  (params (New%20location :type Vector) (New%20rotation :type Rotator) (New%20scale :type Vector))
  (bind _x (Class|KismetMathLibrary|BreakVector3f New%20scale))
  (Variables|Default|SetMPC_WindIntensity (* _x (Variables|Default|GetMPC_WindIntensity)))
  (Utilities|FlowControl|Sequence
    (:then_0
      (Utilities|FlowControl|Delay 2.0)
      (CallFunction|StartWind)
      (for _array_element (Variables|Default|GetCloudParticle)
        (Components|Activation|SetActive (Variables|/Script/Niagara.NiagaraActor|GetNiagaraComponent _array_element) true false)))
    (:then_1
      (for _array_element_2 (Variables|Default|GetCloudParticle)
        (Effects|Components|ParticleSystem|SetFloatParameter (Variables|/Script/Niagara.NiagaraActor|GetNiagaraComponent _array_element_2) "OverallScale" _x)
        (Effects|Components|ParticleSystem|SetVectorParameter (Variables|/Script/Niagara.NiagaraActor|GetNiagaraComponent _array_element_2) "OverallScaleV" New%20scale)))))

(event Custom|StartWind
  (Variables|Default|SetMPC_WindDirection (Math|Vector|Normalize (Math|Vector|MakeVector (Math|Random|RandomFloat) (Math|Random|RandomFloat) 0.0)))
  (Rendering|Material|SetVectorParameterValue "/Game/PlayGround/Epcot/City/Easter_Island/Source/Grass_Clumps_02/Foliage/MPC_GrassWind.MPC_GrassWind" "Wind Vector" (Math|Conversions|ToLinearColor(Vector) (Variables|Default|GetMPC_WindDirection)) :!class /Script/Engine.KismetMaterialLibrary)
  (for _array_element (Variables|Default|GetCloudParticle)
    (Effects|Components|ParticleSystem|SetVectorParameter (Variables|/Script/Niagara.NiagaraActor|GetNiagaraComponent _array_element) "WindSpeed" (* (- (Transformation|GetActorForwardVector) (Transformation|GetActorRightVector)) (Variables|Default|GetParticleWindSpeedIntensity))))
  (Components|Timeline|SetPlayRate (Variables|Default|GetTimeline_Wind) (Math|Random|RandomFloat))
  (bind _intensityscale (Timeline|Timeline_Wind PlayFromStart)
    (:Update
      (Rendering|Material|SetScalarParameterValue "/Game/PlayGround/Epcot/City/Easter_Island/Source/Grass_Clumps_02/Foliage/MPC_GrassWind.MPC_GrassWind" "Wind Intensity" (* _intensityscale (Variables|Default|GetMPC_WindIntensity)) :!class /Script/Engine.KismetMaterialLibrary))
    (:Finished
      (Utilities|Time|SetTimerbyEvent (delegate Custom|StartWind) 4.0 false 1.0 2.0))))

(event EventBeginPlay
  (Utilities|FlowControl|Sequence
    (:then_0
      (bind _returnvalue (Rendering|Material|GetScalarParameterValue "/Game/PlayGround/Epcot/City/Easter_Island/Source/Grass_Clumps_02/Foliage/MPC_GrassWind.MPC_GrassWind" "Wind Intensity" :!class /Script/Engine.KismetMaterialLibrary))
      (bind _output_get (Variables|Default|SetMPC_WindIntensity _returnvalue))
      (Variables|Default|SetMPC_WindIntensity_Original _output_get))
    (:then_1
      (EventDispatchers|AssignOnEarthCitySizeChanged (Variables|Default|GetEarthCitySizeControlComponent) (delegate Custom|OnEarthCitySizeChanged_Event)))))

(event EventEndPlay
  (params (EndPlayReason :type EEndPlayReason%20Enum :default "Destroyed"))
  (Rendering|Material|SetScalarParameterValue "/Game/PlayGround/Epcot/City/Easter_Island/Source/Grass_Clumps_02/Foliage/MPC_GrassWind.MPC_GrassWind" "Wind Intensity" (Variables|Default|GetMPC_WindIntensity_Original) :!class /Script/Engine.KismetMaterialLibrary)
  (Rendering|Material|SetVectorParameterValue "/Game/PlayGround/Epcot/City/Easter_Island/Source/Grass_Clumps_02/Foliage/MPC_GrassWind.MPC_GrassWind" "Wind Vector" (Math|Conversions|ToLinearColor(Vector) (Math|Vector|MakeVector 0.0 0.0 0.0)) :!class /Script/Engine.KismetMaterialLibrary))

(fn ConstructionScript)